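; Shooter game mode Blueprint that manages the on-screen weapon widgets and the gun store widget.
; BeginPlay fills ID-keyed maps of weapon names and widget classes, then pre-creates each game widget hidden in the viewport.
; Switching weapon widgets toggles visibility, hiding the previous ID and showing the new one.
; The store widget is created on demand, sets CanBuyGun on ShooterPC, and is removed by DestroyWidget.
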(event `self.ReceiveBeginPlay`
  (bind _widgetsnames (`self.WidgetsNames`))
  (bind (_weaponconstants_ak47 _weaponconstants_m4a1 _weaponconstants_empty _weaponconstants_knife) (break `/Game/FPWeapon/Blueprints/GunNameConstants` (`self.WeaponConstants`)))
  (bind _widgetsclasses (`self.WidgetsClasses`))
  (`BlueprintMapLibrary.Map_Clear` (`self.WidgetsInstances`))
  (`BlueprintMapLibrary.Map_Clear` (`self.WidgetsNames`))
  (`BlueprintMapLibrary.Map_Clear` (`self.WidgetsClasses`))
  (`BlueprintMapLibrary.Map_Add` _widgetsnames 0 _weaponconstants_ak47)
  (`BlueprintMapLibrary.Map_Add` _widgetsnames 1 _weaponconstants_m4a1)
  (`BlueprintMapLibrary.Map_Add` _widgetsnames 2 _weaponconstants_empty)
  (`BlueprintMapLibrary.Map_Add` _widgetsnames 3 _weaponconstants_knife)
  (`BlueprintMapLibrary.Map_Add` _widgetsclasses 0 "/Game/UI/Weapons/EmptyWidget.EmptyWidget_C")
  (`BlueprintMapLibrary.Map_Add` _widgetsclasses 1 "/Game/UI/Weapons/DefaultKnifeWidget.DefaultKnifeWidget_C")
  (`BlueprintMapLibrary.Map_Add` _widgetsclasses 2 "/Game/UI/Weapons/AK47GameWidget.AK47GameWidget_C")
  (`BlueprintMapLibrary.Map_Add` _widgetsclasses 3 "/Game/FPWeapon/Widgets/M41A.M41A_C")
  (for _index (range 4)
    (`self.CreateWidget` _index)))

(event `CreateGunStoreWidget`
  (params (WidgetClassName :type "UserWidget Class Reference"))
  (bind _returnvalue (`GameplayStatics.GetPlayerController` 0))
  ;[1 1 1] Manage Gun Widgets  (Store widgets )
  (bind _returnvalue_2 (`|CreateWidget` WidgetClassName _returnvalue))
  (bind _output_get (set `self.GunWidget` _returnvalue_2))
  (`UserWidget.AddToViewport` _output_get 0)
  (bind _asshooter_pc (cast `/Game/Blueprints/Shooter/ShooterPC` _returnvalue))
  (set `/Game/Blueprints/Shooter/ShooterPC.CanBuyGun?` true _asshooter_pc))

(event `DestroyWidget`
  ;[1 1 1] Manage Gun Widgets  (Store widgets )
  (`Widget.RemoveFromParent` (`self.GunWidget`)))

(event `CreateGameWidgets`
  (params (Id :type Integer) (PreviousId :type Integer))
  ;[1 1 1] Manage Game Widgets visibility
  (set `self.WidgetId` Id)
  (`self.HideWidgets` PreviousId)
  (`/Engine/EditorBlueprintResources/StandardMacros.IsValid` (`BlueprintMapLibrary.Map_Find` (`self.WidgetsInstances`) (`self.WidgetId`))
    (:`Is Valid`
      (`Widget.SetVisibility` (`BlueprintMapLibrary.Map_Find` (`self.WidgetsInstances`) (`self.WidgetId`)) "Visible"))))

(fn `CreateWidget`
  (params (Id :type Integer))
  (bind _returnvalue (`|CreateWidget` (`BlueprintMapLibrary.Map_Find` (`self.WidgetsClasses`) Id) (`GameplayStatics.GetPlayerController` 0)))
  (`BlueprintMapLibrary.Map_Add` (`self.WidgetsInstances`) Id _returnvalue)
  (`UserWidget.AddToViewport` _returnvalue 0)
  (`Widget.SetVisibility` _returnvalue "Hidden"))

(fn `HideWidgets`
  (params (Id :type Integer))
  (bind _value (`BlueprintMapLibrary.Map_Find` (`self.WidgetsInstances`) Id))
  (if (> Id -1)
    (`/Engine/EditorBlueprintResources/StandardMacros.IsValid` _value
      (:`Is Valid`
        (`Widget.SetVisibility` _value "Hidden"))
      (:`Is Not Valid`
        (`KismetSystemLibrary.PrintString` "widget that must be hidden is not valid")))))

(fn `UserConstructionScript`)