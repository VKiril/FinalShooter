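; Shooter character child that manages knife and AK47 equipment, combat/idle rotation settings and a blood-effect HUD.
; Spawns duplicate weapons per socket (hand, holster), faking draw and holstering by toggling visibility through swap events.
; BuyGun equips the AK47 once and respawns the shop's weapon via the first ChoseAK47 found.
; Hardwired number keys adjust health and test blood decals, including particle-collision splatters with randomised material frame and size.
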(event `Key|Four`
  (params (Key :type "Key Structure" :default "AnyKey"))
  (:`Pressed`
    (bind _returnvalue (`GameplayStatics.SpawnEmitterAttached` "/Game/Mannequin/Blood/SplatterParticleSystem.SplatterParticleSystem" (`self.Mesh`) "None" (0.0 0.0 150.0)))
    (add `ParticleSystemComponent.OnParticleCollide` _returnvalue (delegate `OnCollideEvent`))))

(event `OnCollideEvent`
  (params (EventName :type Name) (EmitterTime :type "Float (double-precision)") (ParticleTime :type Integer) (Location :type "Vector Structure") (Velocity :type "Vector Structure") (Direction :type "Vector Structure") (Normal :type "Vector Structure") (BoneName :type Name) (PhysMat :type "PhysicalMaterial Object Reference"))
  (bind _returnvalue (`KismetMaterialLibrary.CreateDynamicMaterialInstance` "/Game/Mannequin/Blood/SplatterDecalM.SplatterDecalM"))
  (`MaterialInstanceDynamic.SetScalarParameterValue` _returnvalue "Frame" (`KismetMathLibrary.Conv_IntToDouble` (`KismetMathLibrary.RandomIntegerInRange` 1 11)))
  (`GameplayStatics.SpawnDecalAtLocation` _returnvalue (`KismetMathLibrary.Conv_DoubleToVector` (`KismetMathLibrary.RandomFloatInRange` 1.0 10.0)) Location (`KismetMathLibrary.Conv_VectorToRotator` Normal) 20.0))

(event `Key|One`
  (params (Key :type "Key Structure" :default "AnyKey"))
  (:`Pressed`
    (bind _output_get (set `self.CurrentHealth` (+ (`self.CurrentHealth`) 5.0)))
    (`self.UpdateHealth` _output_get)))

(event `Key|Two`
  (params (Key :type "Key Structure" :default "AnyKey"))
  (:`Pressed`
    (bind _output_get (set `self.CurrentHealth` (- (`self.CurrentHealth`) 5.0)))
    (`self.UpdateHealth` _output_get)))

(event `Key|Three`
  (params (Key :type "Key Structure" :default "AnyKey"))
  (:`Pressed`
    (bind _returnvalue (`KismetMaterialLibrary.CreateDynamicMaterialInstance` "/Game/Mannequin/Blood/BloodMaterial.BloodMaterial"))
    (`GameplayStatics.SpawnDecalAtLocation` _returnvalue null (1.0 1.0 1.0) (`SceneComponent.K2_GetComponentLocation` (`self.Mesh`)) (struct :`Pitch` -90.0) 100.0)))

(event `self.ReceiveBeginPlay`
  ;[1 1 1] Init character
  (`self.EqiupKnife` "/Game/FPWeapon/Blueprints/Defaults/DefaultKnifeTalon.DefaultKnifeTalon_C")
  (bind _returnvalue (`|CreateWidget` "/Game/UI/ScreenWidgets/BloodEffectHUD.BloodEffectHUD_C"))
  (bind _output_get (set `self.BloodEfectReference` _returnvalue))
  (`UserWidget.AddToViewport` _output_get 0))

(event `InputAction|BuyGun`
  (params (Key :type "Key Structure" :default "AnyKey"))
  ;[1 1 1] Buy a gun
  (:`Pressed`
    (if (`self.CanBuyWeapon?`)
      (`/Game/Blueprints/Shooter/ShooterPC.UneqipActorAtAll` (`self.GetPlayerController`))
      (if (not (`self.HasGunAttached?`))
        (set `self.HasGunAttached?` true)
        (`self.EquipWeapon` "/Game/FPWeapon/Blueprints/WeaponStore/AK/AK47.AK47_C")
        (set `self.IsAttachingWeapon?` true)
        (set `self.KeepKnifeInHand?` false)
        (set `/Game/Blueprints/Shooter/ShooterPC.ActiveWeaponIndex` 0 (`self.GetPlayerController`))
        (`self.SetActorHiddenInGame` (`self.HolsterGun`) true)))))

(event `MomentPutWeaponToBack`
  ;[1 1 1] Leave gun from hand and put to back
  (`self.SetActorHiddenInGame` (`self.HolsterGun`) false)
  (`self.SetActorHiddenInGame` (`self.HandGun`) true)
  (set `self.IsAttachingWeapon?` false))

(event `TakeWeaponFromBack`
  ;[1 1 1] Take weapon from back
  (`self.SetActorHiddenInGame` (`self.HolsterGun`) true)
  (`self.SetActorHiddenInGame` (`self.HandGun`) false)
  (set `self.IsTakingWeaponFromBack?` false)
  (set `/Game/Blueprints/Shooter/ShooterPC.IsCombatMode?` true (`self.GetPlayerController`))
  (`self.ManageControllerRotationYaw` true))

(event `ManageControllerRotationYaw`
  (params (UseYaw :type Boolean))
  ;[1 1 1] Manage Yaw usage
  (set `self.bUseControllerRotationYaw` UseYaw))

(fn `AddGun`
  (params (SocketName :type Name) (GunClassName :type "Actor Class Reference"))
  (locals (LocalSocketName :type Name))
  (bind _localsocketname (`local.LocalSocketName`))
  (set `local.LocalSocketName` SocketName)
  (bind _returnvalue (`|SpawnActorFromClass` GunClassName (`SceneComponent.K2_GetComponentToWorld` (`self.Mesh`)) "Undefined" "OverrideRootScale"))
  (switch `name` (`local.LocalSocketName`)
    (:`HandWeapon`
      (bind _asak47 (cast `/Game/FPWeapon/Blueprints/WeaponStore/AK/AK47` _returnvalue)
        (:`then`
          (set `/Game/FPWeapon/Blueprints/WeaponStore/AK/AK47.GunOwner` self _asak47)
          (set `/Game/FPWeapon/Blueprints/WeaponStore/AK/AK47.IsCombatGun?` true _asak47)
          (bind _output_get (set `self.HandGun` _asak47))
          (`self.AttachWeapon` _output_get _localsocketname))
        (:`CastFailed`
          (`KismetSystemLibrary.PrintString` "cast to ak47 failed in ShooterChiled.AddGun"))))
    (:`SpineHolsterWeapon`
      (bind _output_get_2 (set `self.HolsterGun` _returnvalue))
      (`self.AttachWeapon` _output_get_2 _localsocketname))))

(fn `AttachWeapon`
  (params (Weapon :type "Actor Object Reference") (SocketName :type Name))
  (`self.K2_AttachToComponent` Weapon (`self.Mesh`) SocketName "SnapToTarget" "SnapToTarget" "KeepWorld" true))

(fn `EqiupKnife`
  (params (Socket :type "Actor Class Reference"))
  (bind (_socketconstants_hand _socketconstants_spinegunholster _socketconstants_knifecombat _socketconstants_knifedefault _socketconstants_knifeholster) (break `/Game/Blueprints/SocketConstants` (`self.SocketConstants`)))
  (bind _defaulthandknife (`self.DefaultHandKnife`))
  (bind _combathandknife (`self.CombatHandKnife`))
  (bind _returnvalue (`SceneComponent.K2_GetComponentToWorld` (`self.Mesh`)))
  (bind _returnvalue_2 (`|SpawnActorFromClass` Socket _returnvalue "AdjustIfPossibleButAlwaysSpawn" "OverrideRootScale"))
  (set `self.DefaultHandKnife` _returnvalue_2)
  (bind _returnvalue_3 (`|SpawnActorFromClass` Socket _returnvalue "AdjustIfPossibleButAlwaysSpawn" "OverrideRootScale"))
  (set `self.CombatHandKnife` _returnvalue_3)
  (bind _returnvalue_4 (`|SpawnActorFromClass` Socket _returnvalue "AdjustIfPossibleButAlwaysSpawn" "OverrideRootScale"))
  (set `self.HolsterKnife` _returnvalue_4)
  ;[1 1 1] Attach knifes to actor
  (`self.AttachWeapon` (`self.CombatHandKnife`) _socketconstants_knifecombat)
  (`self.AttachWeapon` (`self.DefaultHandKnife`) _socketconstants_knifedefault)
  (`self.AttachWeapon` (`self.HolsterKnife`) _socketconstants_knifeholster)
  ;[1 1 1] Hide Hand Knifes
  (`/Engine/EditorBlueprintResources/StandardMacros.IsValid` _defaulthandknife
    (:`Is Valid`
      (`self.SetActorHiddenInGame` _defaulthandknife true)
      (`/Engine/EditorBlueprintResources/StandardMacros.IsValid` _combathandknife
        (:`Is Valid`
          (`self.SetActorHiddenInGame` _combathandknife true))))))

(fn `EquipWeapon`
  (params (ActorClassName :type "Actor Class Reference"))
  (bind (_socketconstants_hand _socketconstants_spinegunholster) (break `/Game/Blueprints/SocketConstants` (`self.SocketConstants`)))
  (`self.AddGun` _socketconstants_hand ActorClassName)
  (`self.AddGun` _socketconstants_spinegunholster ActorClassName)
  (if (`self.KeepKnifeInHand?`)
    (`self.PutKnifeIntoHolster`))
  (bind _outactors (`GameplayStatics.GetAllActorsOfClass` "/Game/FPWeapon/Blueprints/WeaponStore/AK/ChoseAK47.ChoseAK47_C"))
  (`/Game/FPWeapon/Blueprints/WeaponStore/AK/ChoseAK47.RespawnNewWeapon` (`KismetArrayLibrary.Array_Get` _outactors) 2.0))

(fn `PutKnifeIntoHolster`
  (bind _defaulthandknife (`self.DefaultHandKnife`))
  (bind _combathandknife (`self.CombatHandKnife`))
  (bind _holsterknife (`self.HolsterKnife`))
  (if (not (`Actor.bHidden` _defaulthandknife))
    (`self.SetActorHiddenInGame` _defaulthandknife true))
  (if (not (`Actor.bHidden` _combathandknife))
    (`self.SetActorHiddenInGame` _combathandknife true))
  (`/Engine/EditorBlueprintResources/StandardMacros.IsValid` _holsterknife
    (:`Is Valid`
      (`self.SetActorHiddenInGame` _holsterknife false))
    (:`Is Not Valid`
      (`KismetSystemLibrary.PrintString` "knife instance is not valid "))))

(fn `SetCombatModeDetails`
  (bind (_returnvalue_roll _returnvalue_pitch _returnvalue_yaw) (`KismetMathLibrary.BreakRotator` (`self.K2_GetActorRotation`)))
  (`self.K2_SetActorRelativeRotation` (`KismetMathLibrary.MakeRotator` _returnvalue_roll 0.0 _returnvalue_yaw))
  (set `CharacterMovementComponent.bOrientRotationToMovement` false (`self.CharacterMovement`))
  (set `self.bUseControllerRotationRoll` true))

(fn `SetIdleModeDetails`
  (bind (_returnvalue_roll _returnvalue_pitch _returnvalue_yaw) (`KismetMathLibrary.BreakRotator` (`self.K2_GetActorRotation`)))
  (`self.K2_SetActorRelativeRotation` (`KismetMathLibrary.MakeRotator` _returnvalue_roll _returnvalue_pitch _returnvalue_yaw))
  (set `CharacterMovementComponent.bOrientRotationToMovement` true (`self.CharacterMovement`))
  (set `self.bUseControllerRotationRoll` false))

(fn `TakeKnifeInHand`)

(fn `UserConstructionScript`
  (`parent.UserConstructionScript`))