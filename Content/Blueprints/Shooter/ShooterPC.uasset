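; Shooter player controller that handles weapon selection, attacks and crouching for the possessed ShooterChiledCharacter.
; The WeaponSelect axis cycles game-mode widgets for empty hands, knife or AK47 (gun requires one attached), and a click confirms by unequipping, then arming.
; Otherwise, clicks punch, slash or fire by mode, setting character flags or calling the AK47.
; Automatic fire is a toggled mode using a self-rescheduling timer, cleared on release.
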(event `InputAxis|WeaponSelect`
  (params (AxisValue :type "Float (single-precision)"))
  ;[1 1 1] Manege  Weapons Widgets
  (if (== AxisValue 1.0)
    (bind _output_get (set `self.ActiveWeaponIndex` (`KismetMathLibrary.Clamp` (+ (`self.ActiveWeaponIndex`) (`self.MouseWheelStep`)) 0 (- (`BlueprintMapLibrary.Map_Length` (`/Game/Blueprints/Shooter/ShooterGM.WidgetsNames` (`self.GetGameMode`))) (`self.Offset`)))))
    (`self.ShowWidgetByIndex` _output_get)
    (set `self.MouseWheelStep` 1)
    (elif (== AxisValue -1.0)
      (bind _output_get_2 (set `self.ActiveWeaponIndex` (`KismetMathLibrary.Clamp` (- (`self.ActiveWeaponIndex`) (`self.MouseWheelStep`)) 0 (- (`BlueprintMapLibrary.Map_Length` (`/Game/Blueprints/Shooter/ShooterGM.WidgetsNames` (`self.GetGameMode`))) (`self.Offset`)))))
      (`self.ShowWidgetByIndex` _output_get_2)
      (set `self.MouseWheelStep` 1))))

(event `InputAction|ClickAction`
  (params (Key :type "Key Structure" :default "AnyKey"))
  ;[1 1 1] Perform Click event
  (:`Pressed`
    (if (`self.IsShowingGameWidget?`)
      (`/Game/Blueprints/Shooter/ShooterGM.HideWidgets` (`self.GetGameMode`) (`self.ActiveWeaponIndex`))
      (`self.UneqipActorAtAll`)
      (set `self.MouseWheelStep` 0)
      (switch `int` (`self.ActiveWeaponIndex`)
        (:`0`
          (set `self.ArmingType` "empty"))
        (:`1`
          (`self.TakeKnifeDefaultInHand`))
        (:`2`
          (`self.TakeGunInHand` "ak47")))
      (elif (`self.IsCombatMode?`)
        (if (`self.IsGunAutomaticMode?`)
          (`self.WeaponAutomaticFireMode`)
          (else
            (`self.GunFireFunc`)))
        (elif (`self.IsKeepingKnifeInHand?`)
          (`self.CutTheEnemy`)
          (else
            (`self.Punch`))))))
  (:`Released`
    (`self.Released`)))

(event `InputAction|CrouchAction`
  (params (Key :type "Key Structure" :default "AnyKey"))
  (bind _asshooter_chiled_character (`self.TakeShooterChiledActor`))
  ;[1 1 1] Crouch pose trigger
  (:`Pressed`
    (if (`self.IsCombatMode?`)
      (if (`/Game/Blueprints/Shooter/ShooterChiledCharacter.IsCrouching?` _asshooter_chiled_character)
        (set `/Game/Blueprints/Shooter/ShooterChiledCharacter.IsCrouching?` false _asshooter_chiled_character)
        (else
          (set `/Game/Blueprints/Shooter/ShooterChiledCharacter.IsCrouching?` true _asshooter_chiled_character))))))

(event `InputAction|AutomaticMode`
  (params (Key :type "Key Structure" :default "AnyKey"))
  ;[1 1 1] Wepon Automatic mode triggering
  (:`Pressed`
    (set `self.IsGunAutomaticMode?` (not (`self.IsGunAutomaticMode?`)))))

(event `WeaponAutomaticFireMode`
  (bind _returnvalue (`KismetSystemLibrary.K2_SetTimerDelegate` (delegate `WeaponAutomaticFireMode`) 0.2))
  (`self.GunFireFunc`))

(event `ClearWeaponTimer`
  (`KismetSystemLibrary.K2_ClearAndInvalidateTimerHandle` (stale `WeaponAutomaticFireMode` _returnvalue)))

(fn `CutTheEnemy`
  (set `/Game/Blueprints/Shooter/ShooterChiledCharacter.IsCutting?` true (`self.TakeShooterChiledActor`))
  (`KismetSystemLibrary.PrintString` "cut enemy "))

(fn `GunFireFunc`
  (bind _asak47 (cast `/Game/FPWeapon/Blueprints/WeaponStore/AK/AK47` (`/Game/Blueprints/Shooter/ShooterChiledCharacter.HandGun` (`self.TakeShooterChiledActor`)))
    (:`then`
      (`/Game/FPWeapon/Blueprints/WeaponStore/AK/AK47.Fire` _asak47))
    (:`CastFailed`
      (`KismetSystemLibrary.PrintString` "cast to ak47 failed in ShooterPC.FireEvent"))))

(fn `Punch`
  (set `/Game/Blueprints/Shooter/ShooterChiledCharacter.IsPunching?` true (`self.TakeShooterChiledActor`)))

(fn `Released`
  (if (`self.IsGunAutomaticMode?`)
    (`self.ClearWeaponTimer`))
  (if (not (or (`self.IsShowingGameWidget?`) (`self.IsCombatMode?`)))
    (set `/Game/Blueprints/Shooter/ShooterChiledCharacter.IsPunching?` false (`self.TakeShooterChiledActor`))))

(fn `ShowWidgetByIndex`
  (params (Id :type Integer))
  (locals (LocalId :type Integer))
  (set `local.LocalId` Id)
  (if (< Id 2)
    (`/Game/Blueprints/Shooter/ShooterGM.CreateGameWidgets` (`self.GetGameMode`) (`local.LocalId`) (`self.Previuosid`) :!label _label)
    (set `self.IsShowingGameWidget?` true)
    (set `self.Previuosid` (`local.LocalId`))
    (elif (`/Game/Blueprints/Shooter/ShooterChiledCharacter.HasGunAttached?` (`self.TakeShooterChiledActor`))
      (goto _label)
      (else
        (set `self.ActiveWeaponIndex` 1)))))

(fn `TakeGunInHand`
  (params (GunName :type String))
  (bind _asshooter_chiled_character (`self.TakeShooterChiledActor`))
  (if (`/Game/Blueprints/Shooter/ShooterChiledCharacter.HasGunAttached?` (`self.TakeShooterChiledActor`))
    (set `self.ArmingType` GunName)
    (set `/Game/Blueprints/Shooter/ShooterChiledCharacter.IsTakingWeaponFromBack?` true _asshooter_chiled_character)
    (`/Game/Blueprints/Shooter/ShooterChiledCharacter.SetCombatModeDetails` _asshooter_chiled_character)))

(fn `TakeKnifeDefaultInHand`
  (bind _asshooter_chiled_character (`self.TakeShooterChiledActor`))
  (`self.SetActorHiddenInGame` (`/Game/Blueprints/Shooter/ShooterChiledCharacter.HolsterKnife` _asshooter_chiled_character) true)
  (`self.SetActorHiddenInGame` (`/Game/Blueprints/Shooter/ShooterChiledCharacter.DefaultHandKnife` _asshooter_chiled_character) false)
  (set `self.ArmingType` "knife")
  (set `self.IsKeepingKnifeInHand?` true))

(fn `UneqipActorAtAll`
  (bind _asshooter_chiled_character (`self.TakeShooterChiledActor`))
  (bind _asshooter_chiled_character_2 (`self.TakeShooterChiledActor`))
  (`/Game/Blueprints/Shooter/ShooterChiledCharacter.SetIdleModeDetails` _asshooter_chiled_character_2)
  (`/Game/Blueprints/Shooter/ShooterChiledCharacter.ManageControllerRotationYaw` _asshooter_chiled_character_2 false)
  (set `self.IsShowingGameWidget?` false)
  (switch `string` (`self.ArmingType`)
    (:`knife`
      (`self.SetActorHiddenInGame` (`/Game/Blueprints/Shooter/ShooterChiledCharacter.HolsterKnife` _asshooter_chiled_character) false)
      (`self.SetActorHiddenInGame` (`/Game/Blueprints/Shooter/ShooterChiledCharacter.DefaultHandKnife` _asshooter_chiled_character) true)
      (`self.SetActorHiddenInGame` (`/Game/Blueprints/Shooter/ShooterChiledCharacter.CombatHandKnife` _asshooter_chiled_character) true)
      (set `self.IsKeepingKnifeInHand?` false))
    (:`ak47`
      (set `self.IsCombatMode?` false)
      (set `/Game/Blueprints/Shooter/ShooterChiledCharacter.IsAttachingWeapon?` true (`self.TakeShooterChiledActor`)))))

(fn `UserConstructionScript`
  (bind _weaponstype (`self.WeaponsType`))
  (`BlueprintMapLibrary.Map_Add` _weaponstype 0 "empty")
  (`BlueprintMapLibrary.Map_Add` _weaponstype 1 "knife")
  (`BlueprintMapLibrary.Map_Add` _weaponstype 2 "gun"))