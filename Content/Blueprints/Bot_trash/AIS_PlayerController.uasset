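; Player controller that moves a stored pawn along control-rotation axes on the horizontal plane and handles mouse click and hold input.
; Movement input offsets the pawn without sweep and aligns its ControllerArrow to control rotation.
; Tick feeds per-button gates whose short timers separate clicks from holds, though nothing here re-arms the click flags.
; Right hold rotates control yaw and the spring arm; left hold and both clicks only print debug text.
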(event `InputAxis|MoveForward`
  (params (AxisValue :type "Float (single-precision)"))
  (bind _returnvalue (`self.GetControlRotation`))
  (`self.K2_AddActorLocalOffset` (`self.StorePawn`) (* (* (+ (* (`KismetMathLibrary.GetForwardVector` _returnvalue) AxisValue) (* (`KismetMathLibrary.GetRightVector` _returnvalue) (stale `InputAxis|MoveRight` AxisValue))) (`self.MovementRate`)) (1.0 1.0 0.0)) false false :!label _label)
  (`SceneComponent.K2_SetWorldRotation` (`/Game/Blueprints/Bot_trash/AIS_PlayerPawn.ControllerArrow` (`self.StorePawn`)) (`self.GetControlRotation`) false false))

(event `InputAxis|MoveRight`
  (params (AxisValue :type "Float (single-precision)"))
  (goto _label))

(event `Key|LeftMouseButton`
  (params (Key :type "Key Structure" :default "AnyKey"))
  (bind _leftclickholdcounter (`self.LeftClickHoldCounter`))
  (:`Pressed`
    (goto _label_2 :!via `Open`))
  (:`Released`
    (if (not (not (`self.LeftClick`)))
      (`KismetSystemLibrary.PrintString` "left click "))
    (set `self.LeftClickHoldCounter` 0.0)
    (set `self.LeftClick` false)
    (goto _label_2 :!via `Close`)))

(event `self.ReceiveTick`
  (params (DeltaSeconds :type "Float (single-precision)"))
  (bind (_returnvalue_roll _returnvalue_pitch _returnvalue_yaw) (`KismetMathLibrary.BreakRotator` (`self.GetControlRotation`)))
  (bind _leftclickholdcounter (`self.LeftClickHoldCounter`))
  (bind _rightclickholdcounter (`self.RightClickHoldCounter`))
  (bind _springarm (`/Game/Blueprints/Bot_trash/AIS_PlayerPawn.SpringArm` (`self.StorePawn`)))
  (bind (_returnvalue_roll_2 _returnvalue_pitch_2 _returnvalue_yaw_2) (`KismetMathLibrary.BreakRotator` (`SceneComponent.K2_GetComponentRotation` _springarm)))
  (`|ExecutionSequence`
    (:`then_0`
      (`/Engine/EditorBlueprintResources/StandardMacros.Gate` true :!label _label_2
        (:`Exit`
          (if (`self.LeftClick`)
            (if (>= _leftclickholdcounter 0.12)
              (set `self.LeftClick` false)
              (else
                (set `self.LeftClickHoldCounter` (+ DeltaSeconds _leftclickholdcounter))))
            (else
              (`KismetSystemLibrary.PrintString` "left mouse hold"))))))
    (:`then_1`
      (`/Engine/EditorBlueprintResources/StandardMacros.Gate` true :!label _label_3
        (:`Exit`
          (if (`self.RightClick`)
            (if (>= _rightclickholdcounter 0.12)
              (set `self.RightClick` false)
              (else
                (set `self.RightClickHoldCounter` (+ DeltaSeconds _rightclickholdcounter))))
            (else
              (`self.SetControlRotation` (`KismetMathLibrary.MakeRotator` 0.0 0.0 (+ (`self.GetInputAxisKeyValue`) _returnvalue_yaw)))
              (`SceneComponent.K2_SetWorldRotation` _springarm (`KismetMathLibrary.MakeRotator` 0.0 (+ (`self.GetInputAxisKeyValue`) _returnvalue_pitch_2) (+ (`self.GetInputAxisKeyValue`) _returnvalue_yaw_2)) false false))))))))

(event `Key|RightMouseButton`
  (params (Key :type "Key Structure" :default "AnyKey"))
  (:`Pressed`
    (goto _label_3 :!via `Open`))
  (:`Released`
    (if (not (not (`self.RightClick`)))
      (`KismetSystemLibrary.PrintString` "right click "))
    (set `self.RightClickHoldCounter` 0.0)
    (set `self.RightClick` false)
    (goto _label_3 :!via `Close`)))

(fn `UserConstructionScript`)