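; Gun store display actor for the M4A1 Maveric that shows a weapon widget while something overlaps its Box.
; The construction script fills a hardcoded characteristics struct and converts it into a text version with units appended.
; Box begin overlap creates an M41A widget and adds it to the viewport.
; End overlap only hides that widget, so each new overlap creates another instance.
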(event `self.ReceiveBeginPlay`)

(event `self.ReceiveActorBeginOverlap`
  (params (OtherActor :type "Actor Object Reference")))

(event `self.ReceiveTick`
  (params (DeltaSeconds :type "Float (single-precision)")))

(event `self.Box.OnComponentBeginOverlap`
  (params (OtherActor :type "Actor Object Reference") (OtherComp :type "PrimitiveComponent Object Reference") (OtherBodyIndex :type Integer) (bFromSweep :type Boolean) (SweepResult :type "HitResult Structure (by ref)"))
  (bind _returnvalue (`|CreateWidget` "/Game/FPWeapon/Widgets/M41A.M41A_C"))
  (bind _output_get (set `self.WeaponWidgeReference` _returnvalue))
  (`UserWidget.AddToViewport` _output_get 0))

(event `self.Box.OnComponentEndOverlap`
  (params (OtherActor :type "Actor Object Reference") (OtherComp :type "PrimitiveComponent Object Reference") (OtherBodyIndex :type Integer))
  (`Widget.SetVisibility` (`self.WeaponWidgeReference`) "Hidden"))

(fn `UserConstructionScript`
  (bind _output_get (set `self.GunCharacteristics` (make `/Game/FPWeapon/Blueprints/GUN_STORE/GunDescription` "M4A1 Maveric" 220 "$" 1200 "mm" 450 30 3700 5 "g" 5)))
  (set `self.GunCharacteristicsString` (make `/Game/FPWeapon/Blueprints/GUN_STORE/GunDescriptionString` (`KismetTextLibrary.Conv_StringToText` (break `/Game/FPWeapon/Blueprints/GUN_STORE/GunDescription` _output_get)) (`KismetTextLibrary.Conv_StringToText` (`KismetStringLibrary.Concat_StrStr` (`KismetStringLibrary.Conv_IntToString` (`.Price_60_9B7D3C204B7F87D4C07033B2CA1CA34B` (break `/Game/FPWeapon/Blueprints/GUN_STORE/GunDescription` _output_get))) (`.PriceUOM_39_66C73C6845F58A1FF372758E57ACA155` (break `/Game/FPWeapon/Blueprints/GUN_STORE/GunDescription` _output_get)))) "" (`KismetTextLibrary.Conv_StringToText` (`KismetStringLibrary.Concat_StrStr` (`KismetStringLibrary.Conv_IntToString` (`.ArmLenght_61_A5B318FA478D9DD8D9E952B374EA1599` (break `/Game/FPWeapon/Blueprints/GUN_STORE/GunDescription` _output_get))) (`.LenghtUOM_55_E35F0D4D4317A6B6A64E6F9723DCA6B2` (break `/Game/FPWeapon/Blueprints/GUN_STORE/GunDescription` _output_get)))) "" (`KismetTextLibrary.Conv_StringToText` (`KismetStringLibrary.Concat_StrStr` (`KismetStringLibrary.Conv_IntToString` (`.PipeLenght_62_F3E42A3F48EEB144A56B8BA943CF9C07` (break `/Game/FPWeapon/Blueprints/GUN_STORE/GunDescription` _output_get))) (`.LenghtUOM_55_E35F0D4D4317A6B6A64E6F9723DCA6B2` (break `/Game/FPWeapon/Blueprints/GUN_STORE/GunDescription` _output_get)))) (`KismetTextLibrary.Conv_IntToText` (`.MagazineCapacity_45_575DDBFC4A079D4269D82D98B20C8C5D` (break `/Game/FPWeapon/Blueprints/GUN_STORE/GunDescription` _output_get))) (`KismetTextLibrary.Conv_StringToText` (`KismetStringLibrary.Concat_StrStr` (`KismetStringLibrary.Conv_IntToString` (`.WeightWithoutCartridge_63_BE9E866E433055ECA42FFE85349821DA` (break `/Game/FPWeapon/Blueprints/GUN_STORE/GunDescription` _output_get))) (`.WeightUOM_54_1C0110C944631E571CDB90A38BCCB13A` (break `/Game/FPWeapon/Blueprints/GUN_STORE/GunDescription` _output_get)))) (`KismetTextLibrary.Conv_StringToText` (`KismetStringLibrary.Concat_StrStr` (`KismetStringLibrary.Conv_IntToString` (`.BulletWeight_64_F0DF35AC438AB100BF00BAA5258C15DB` (break `/Game/FPWeapon/Blueprints/GUN_STORE/GunDescription` _output_get))) (`.WeightUOM_54_1C0110C944631E571CDB90A38BCCB13A` (break `/Game/FPWeapon/Blueprints/GUN_STORE/GunDescription` _output_get)))) "" (`KismetTextLibrary.Conv_IntToText` (`.Calber_65_E13071ED4656693A0FEA5389E14BC28A` (break `/Game/FPWeapon/Blueprints/GUN_STORE/GunDescription` _output_get))))))