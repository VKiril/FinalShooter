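; DefaultKnifeTalon is a knife actor in the FPWeapon content that reacts to hitting a surface like a paintball projectile.
; On Hit it spawns a randomly sized paint splat decal aligned to the surface normal, using a dynamic material to randomize frame and color.
; It pushes physics-simulating components with an impulse scaled from its velocity, prints a debug string, and destroys itself.
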(event `self.ReceiveHit`
  (params (MyComp :type "PrimitiveComponent Object Reference") (Other :type "Actor Object Reference") (OtherComp :type "PrimitiveComponent Object Reference") (bSelfMoved :type Boolean) (HitLocation :type "Vector Structure") (HitNormal :type "Vector Structure") (NormalImpulse :type "Vector Structure") (Hit :type "HitResult Structure (by ref)"))
  (`KismetSystemLibrary.PrintString` "*******cut amd draw")
  (bind _returnvalue (`GameplayStatics.SpawnDecalAtLocation` "/Game/BulletDecals/PaintSplat_M.PaintSplat_M" (`KismetMathLibrary.Conv_DoubleToVector` (`KismetMathLibrary.RandomFloatInRange` 15.0 30.0)) HitLocation (`KismetMathLibrary.Conv_VectorToRotator` HitNormal)))
  (bind _returnvalue_2 (`DecalComponent.CreateDynamicMaterialInstance` _returnvalue))
  (`MaterialInstanceDynamic.SetScalarParameterValue` _returnvalue_2 "Frame" (`KismetMathLibrary.Conv_IntToDouble` (`KismetMathLibrary.RandomIntegerInRange` 0 3)))
  (`MaterialInstanceDynamic.SetVectorParameterValue` _returnvalue_2 "Color" (`KismetMathLibrary.MakeColor` (`KismetMathLibrary.RandomFloatInRange` 0.0 1.0) (`KismetMathLibrary.RandomFloatInRange` 0.0 1.0) (`KismetMathLibrary.RandomFloatInRange` 0.0 1.0) (`KismetMathLibrary.RandomFloatInRange` 0.6 0.8)))
  (if (`SceneComponent.IsSimulatingPhysics` OtherComp "None")
    (`PrimitiveComponent.AddImpulseAtLocation` OtherComp (* (`self.GetVelocity`) 100) (`self.K2_GetActorLocation`) "None"))
  (`self.K2_DestroyActor` self))

(fn `UserConstructionScript`)