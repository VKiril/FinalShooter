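; Gun actor that fires Bullet actors in single or automatic fire and shows indicators for combat and automatic mode.
; Each shot spawns a bullet at the Arrow component's transform, with an attached gunshot sound and muzzle flash on the skeletal mesh.
; Automatic fire repeats on a looping timer that the shoot-end event clears.
; A yaw-offset bullet transform helper is defined but not used by the firing path.
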(event `self.ReceiveBeginPlay`
  (`SceneComponent.SetVisibility` (`self.Mode`) false false)
  (`SceneComponent.SetVisibility` (`self.PowenOn`) false false))

(event `/Game/FPWeapon/Blueprints/GunInterface.SetCombatMode`
  (`SceneComponent.SetVisibility` (`self.PowenOn`) true false))

(event `/Game/FPWeapon/Blueprints/GunInterface.UnsetCombatMode`
  (`SceneComponent.SetVisibility` (`self.PowenOn`) false false)
  (`SceneComponent.SetVisibility` (`self.Mode`) false false))

(event `/Game/FPWeapon/Blueprints/GunInterface.ShootAutimaticMode`
  (bind _arrow (`self.Arrow`))
  (bind _returnvalue (`KismetSystemLibrary.K2_SetTimerDelegate` (delegate `/Game/FPWeapon/Blueprints/GunInterface.ShootAutimaticMode`) 0.1 true))
  (set `self.AutomaticModeTimer` _returnvalue)
  (`|ExecutionSequence` :!label _label
    (:`then_0`
      (`GameplayStatics.SpawnSoundAttached` "/Game/FPWeapon/Sound/Gun+Shot2.Gun+Shot2" (`self.SkeletalMesh`)))
    (:`then_1`
      (`|SpawnActorFromClass` "/Game/FPWeapon/Blueprints/Bullet.Bullet_C" (`SceneComponent.K2_GetComponentToWorld` (`self.Arrow`)) "Undefined" "OverrideRootScale")
      (`GameplayStatics.SpawnEmitterAttached` "/Game/FPWeapon/Particles/GunFire.GunFire" (`self.SkeletalMesh`) "explosion" (`SceneComponent.GetUpVector` _arrow) (`SceneComponent.RelativeRotation` _arrow)))))

(event `/Game/FPWeapon/Blueprints/GunInterface.ShootEventStart`
  (goto _label))

(event `/Game/FPWeapon/Blueprints/GunInterface.ShootEventEnd`
  (`KismetSystemLibrary.K2_ClearTimerHandle` (`self.AutomaticModeTimer`)))

(event `/Game/FPWeapon/Blueprints/GunInterface.SetAutomaticMode`
  (`SceneComponent.SetVisibility` (`self.Mode`) true false))

(event `/Game/FPWeapon/Blueprints/GunInterface.UnsetAutomaticMode`
  (`SceneComponent.SetVisibility` (`self.Mode`) false false))

(fn `functionMakeBulletTransform`
  (returns (transform :type "Transform Structure"))
  (bind _returnvalue (`SceneComponent.K2_GetComponentToWorld` (`self.SkeletalMesh`)))
  (return (`KismetMathLibrary.MakeTransform` (.location _returnvalue) (`KismetMathLibrary.MakeRotator` (.roll (.rotation _returnvalue)) (.pitch (.rotation _returnvalue)) (+ (.yaw (.rotation _returnvalue)) 90.0)) (.scale _returnvalue))))

(fn `UserConstructionScript`)